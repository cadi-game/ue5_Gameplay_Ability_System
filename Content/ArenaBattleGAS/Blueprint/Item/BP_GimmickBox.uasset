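; BP_GimmickBox is a one-shot trigger box that marks a gimmick or the game as cleared through gameplay tags.
; On overlap it disables its trigger and adds a loose, non-replicated cleared tag to TargetGimmick, chosen by the GameCleared flag.
; When GameCleared is set, BeginPlay makes the player pawn that target.
; Trigger overlap also activates an effect, and the actor destroys itself when that effect finishes.
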(event OnSystemFinished(Effect)
  (params (PSystem :type Particle%20System%20Component%20Object%20Reference))
  (Actor|DestroyActor))

(event OnComponentBeginOverlap(Trigger)
  (params (OverlappedComponent :type Primitive%20Component%20Object%20Reference) (OtherActor :type Actor%20Object%20Reference) (OtherComp :type Primitive%20Component%20Object%20Reference) (OtherBodyIndex :type Integer) (bFromSweep :type Boolean) (SweepResult :type Hit%20Result%20Structure%20%28by%20ref%29))
  (Components|Activation|Activate (Variables|Default|GetEffect) false))

(event Collision|EventActorBeginOverlap
  (params (OtherActor :type Actor%20Object%20Reference))
  (Collision|SetCollisionEnabled (Variables|Default|GetTrigger) "NoCollision")
  (Utilities|IsValid (Variables|Default|GetTargetGimmick)
    (:Is%20Valid
      (Ability|GameplayEffect|AddLooseGameplayTags (Variables|Default|GetTargetGimmick) (select (Variables|Default|GetGameCleared) (GameplayTags|MakeGameplayTagContainerfromTag "(TagName=\"Event.Game.Cleared\")") (GameplayTags|MakeGameplayTagContainerfromTag "(TagName=\"Event.Gimmick.Cleared\")"))))))

(event EventTick
  (params (DeltaSeconds :type Float%20%28single-precision%29))
  (|CallParentFunction DeltaSeconds) ; This node is disabled and will not be called.\nDrag off pins to build functionality.
)

(event EventBeginPlay
  (if (Variables|Default|GetGameCleared)
    (Variables|Default|SetTargetGimmick (Game|Player|GetPlayerPawn 0))))

(fn ConstructionScript
  (|CallParentFunction))